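; Zombie enemy that chases a player-controlled pawn and melee-attacks it until its HP runs out and it is destroyed.
; ChasePlayer uses AI MoveTo on a target picked by index from the game mode's controllers, then loops an attack montage, resuming pursuit when out of range.
; AttackTrace, intended for an AnimNotify, sphere-traces ahead to damage player characters.
; CurHP's RepNotify updates a widget health bar, which a timer turns toward the local camera.
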(event `self.ReceiveBeginPlay`
  (bind _output_get (set `self.MaxHP` 100.0))
  (set `self.CurHP` _output_get)
  (`KismetSystemLibrary.Delay` 0.5)
  (`KismetSystemLibrary.K2_SetTimer` null "HPLookAtPlayer" 0.2 true))

(event `ChasePlayer`
  ;[1 1 1] 플레이어 쫓기
  (`/Engine/EditorBlueprintResources/StandardMacros.IsValid` (`self.ChaseChar`)
    (:`Is Valid`
      (`|AIMoveTo` self (0.0 0.0 0.0) (`self.ChaseChar`) 110.0
        (:`OnSuccess`
          (`self.Attack`))))
    (:`Is Not Valid`
      (`self.SetChar`))))

(event `SetChar`
  ;[1 1 1] 쫓을 플레이어 설정
  (`/Engine/EditorBlueprintResources/StandardMacros.IsValid` (`self.ChaseChar`)
    (:`Is Not Valid`
      (set `self.ChaseChar` (`Controller.K2_GetPawn` (`|GetArrayItem` (`/Game/Blueprints/Game/BP_GamePlayGM.AllPlayerControllers` (cast `/Game/Blueprints/Game/BP_GamePlayGM` (`GameplayStatics.GetGameMode`) :!pure true)) (`self.ChaseIndex`))))
      (`self.SetChar`))))

(event `Attack`
  ;[1 1 1] 플레이어 공격
  (`self.K2_SetActorRotation` (`KismetMathLibrary.FindLookAtRotation` (`self.K2_GetActorLocation` self) (`self.K2_GetActorLocation` (`self.ChaseChar`))))
  (`self.PlayAttackMontange`))

(event `PlayAttackMontange`
  ;[1 1 1] 적 공격 애니메이션
  (`|PlayMontage` (`self.Mesh`) "/Game/Zombie/Animation/Zombie_Attack_Montage.Zombie_Attack_Montage" 3.0
    (:`OnCompleted`
      (if (> (`KismetMathLibrary.Vector_Distance` (`self.K2_GetActorLocation` self) (`self.K2_GetActorLocation` (`self.ChaseChar`))) 150.0)
        (`self.ChasePlayer`)
        (else
          (`self.Attack`))))))

(event `AttackTrace`
  (bind _returnvalue (`self.K2_GetActorLocation`))
  (bind _returnvalue_2 (`KismetMathLibrary.GetForwardVector` (`self.K2_GetActorRotation`)))
  ;[1 1 1] AnimNotify로 불러올 함수내용
  (bind (_outhit _returnvalue_3) (`KismetSystemLibrary.SphereTraceSingleForObjects` :`Start` (+ _returnvalue (* _returnvalue_2 100.0)) :`End` (+ _returnvalue (* _returnvalue_2 170.0)) :`Radius` 30.0 :`ObjectTypes` (`|MakeArray` "ObjectTypeQuery3" :!type "EObjectTypeQuery Enum") :`DrawDebugType` "ForDuration"))
  (if _returnvalue_3
    (bind (_bblockinghit _binitialoverlap _time _distance _location _impactpoint _normal _impactnormal _physmat _hitactor) (`GameplayStatics.BreakHitResult` _outhit))
    (bind _asbp_third_person_character (cast `/Game/ThirdPerson/Blueprints/BP_ThirdPersonCharacter` _hitactor))
    (`KismetSystemLibrary.PrintString` (`KismetSystemLibrary.GetDisplayName` _asbp_third_person_character))
    (`GameplayStatics.ApplyDamage` _hitactor 10.0)))

(event `SetHp`
  (params (GetDamage :type "Float (double-precision)"))
  (bind _output_get (set `self.CurHP` (- (`self.CurHP`) GetDamage)))
  (if (<= _output_get 0.0)
    (`self.K2_DestroyActor`)))

(event `self.ReceiveEndPlay`
  (params (EndPlayReason :type "EEndPlayReason Enum" :default "Destroyed")))

(fn `HPLookAtPlayer`
  (`SceneComponent.K2_SetWorldRotation` (`self.HpWidget`) (`KismetMathLibrary.FindLookAtRotation` (`SceneComponent.K2_GetComponentLocation` (`self.HpWidget`)) (`self.K2_GetActorLocation` (`GameplayStatics.GetPlayerCameraManager` 0))) false false))

(fn `OnRep_CurHP`
  (bind _returnvalue (`WidgetComponent.GetWidget` (`self.HpWidget`)))
  (`/Engine/EditorBlueprintResources/StandardMacros.IsValid` _returnvalue
    (:`Is Valid`
      (bind _ashptag_widget (cast `/Game/Zombie/Widget/HPTagWidget` _returnvalue))
      (`/Game/Zombie/Widget/HPTagWidget.SetHp` _ashptag_widget (/ (`self.CurHP`) (`self.MaxHP`))))
    (:`Is Not Valid`
      (`KismetSystemLibrary.K2_SetTimer` null "OnRep_CurHP"))))

(fn `SetWidgetRef`
  (bind _returnvalue (`WidgetComponent.GetWidget` (`self.HpWidget`)))
  (`/Engine/EditorBlueprintResources/StandardMacros.IsValid` _returnvalue
    (:`Is Valid`
      (bind _ashptag_widget (cast `/Game/Zombie/Widget/HPTagWidget` _returnvalue))
      (set `self.HPTagWidgetRef` _ashptag_widget))
    (:`Is Not Valid`
      (`KismetSystemLibrary.K2_SetTimer` null "SetWidgetRef" 0.1))))

(fn `UserConstructionScript`)